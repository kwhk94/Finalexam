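; HeroBP is the player hero, a cursor-aimed character with axis movement, punching and a rifle mode.
; It faces its velocity until a shot, when clicking moves a spawned marker to the cursor hit and turns the hero toward it.
; Without a rifle, clicking sets a punch flag, with spheres attached to both hand sockets.
; MakeRifle spawns and attaches a gun and switches to the rifle animation Blueprint.
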(event `self.ReceiveBeginPlay`
  (bind _returnvalue (`|SpawnActorFromClass` "/Game/UI/MousePointBP.MousePointBP_C" (`KismetMathLibrary.Conv_VectorToTransform` (`self.K2_GetActorLocation`)) "Undefined" "OverrideRootScale"))
  (set `self.MouseClickPoint` _returnvalue)
  (set `PlayerController.bShowMouseCursor` true (`GameplayStatics.GetPlayerController` 0)))

(event `InputAxis|forward`
  (params (AxisValue :type "Float (single-precision)"))
  (`self.AddMovementInput` (10.0 0.0 0.0) AxisValue))

(event `InputAxis|rightleft`
  (params (AxisValue :type "Float (single-precision)"))
  (`self.AddMovementInput` (0.0 -10.0 0.0) AxisValue))

(event `self.ReceiveTick`
  (params (DeltaSeconds :type "Float (single-precision)"))
  (if (not (`self.shot`))
    (`self.K2_SetActorRotation` (`KismetMathLibrary.MakeRotator` 0.0 0.0 (.yaw (`KismetMathLibrary.Conv_VectorToRotator` (`MovementComponent.Velocity` (`self.CharacterMovement`))))))))

(event `InputAction|LeftMouseClicked`
  (params (Key :type "Key Structure" :default "AnyKey"))
  (bind (_returnvalue_roll _returnvalue_pitch _returnvalue_yaw) (`KismetMathLibrary.BreakRotator` (`KismetMathLibrary.FindLookAtRotation` (`SceneComponent.K2_GetComponentLocation` (`self.CapsuleComponent`)) (`SceneComponent.K2_GetComponentLocation` (`/Game/UI/MousePointBP.DefaultSceneRoot` (`self.MouseClickPoint`))))))
  (:`Pressed`
    (if (`self.RifleOnOff`)
      (`self.K2_SetActorLocation` (`self.MouseClickPoint`) (`.Location` (`GameplayStatics.BreakHitResult` (`PlayerController.GetHitResultUnderCursorByChannel` (`GameplayStatics.GetPlayerController` 0) "TraceTypeQuery1" true))) false false)
      (bind _output_get (set `self.rotation` (`KismetMathLibrary.MakeRotator` 0.0 0.0 _returnvalue_yaw)))
      (`self.K2_SetActorRotation` _output_get)
      (set `self.shot` true)
      (else
        (set `self.IsPunching?` true)
        (`SkeletalMeshComponent.SetAnimInstanceClass` (`self.Mesh`) "/Game/Hero/HeroAnimBP.HeroAnimBP_C"))))
  (:`Released`
    (if (not (`self.RifleOnOff`))
      (set `self.IsPunching?` false))))

(fn `MakeRifle`
  (set `self.RifleOnOff` true)
  (`SkeletalMeshComponent.SetAnimInstanceClass` (`self.Mesh`) "/Game/Hero/HeroRifleAnimBP.HeroRifleAnimBP_C")
  (bind _returnvalue (`|SpawnActorFromClass` "/Game/Gun/Gun.Gun_C" (`SceneComponent.K2_GetComponentToWorld` (`self.Mesh`)) "Undefined" "OverrideRootScale"))
  (bind _output_get (set `self.Gun` _returnvalue))
  (`self.K2_AttachToComponent` _output_get (`self.Mesh`) "GunSocket" "SnapToTarget" "SnapToTarget" "KeepRelative" true))

(fn `UserConstructionScript`
  (`SceneComponent.K2_AttachToComponent` (`self.r_Sphere`) (`self.Mesh`) "hand_r" "SnapToTarget" "SnapToTarget" "KeepRelative" true)
  (`SceneComponent.K2_AttachToComponent` (`self.l_Sphere`) (`self.Mesh`) "hand_l" "SnapToTarget" "SnapToTarget" "KeepRelative" true))